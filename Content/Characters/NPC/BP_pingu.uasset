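; Penguin NPC character that reacts to seeing the player, driven through an AI Blackboard.
; It sets a slow walk speed on BeginPlay.
; When PawnSensing sees the BP_ThirdPersonCharacter, it writes that pawn's location to JG_posicion, turns on "asustado" (scared) and clears "alerta" (alert).
; This file only writes those keys and never resets them; the resulting behavior is defined outside it.
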(event `self.ReceiveBeginPlay`
  (set `CharacterMovementComponent.MaxWalkSpeed` 100.0 (`self.CharacterMovement`)))

(event `self.PawnSensing.OnSeePawn`
  (params (Pawn :type "Pawn Object Reference"))
  (bind _returnvalue (`AIBlueprintHelperLibrary.GetBlackboard` null))
  (bind _returnvalue_2 (`GameplayStatics.GetActorOfClass` "/Game/ThirdPerson/Blueprints/BP_ThirdPersonCharacter.BP_ThirdPersonCharacter_C"))
  (if (== _returnvalue_2 Pawn)
    (`BlackboardComponent.SetValueAsVector` _returnvalue "JG_posicion" (`self.K2_GetActorLocation` Pawn))
    (`BlackboardComponent.SetValueAsBool` _returnvalue "asustado" true)
    (`BlackboardComponent.SetValueAsBool` _returnvalue "alerta" false)))

(fn `UserConstructionScript`)